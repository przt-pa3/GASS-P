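; Gameplay ability that switches which equipment slot the character has armed, or disarms the current item.
; On activation with authority, it gets the character's GASS equipment manager component and uses the ability level as the selector.
; A negative level calls DisarmItem, while other levels index LevelEquipIndexMapping to pick the slot passed to ChangeArmItem.
; The ability then ends immediately, with or without authority.
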(event `self.K2_ActivateAbility`
  (bind _returnvalue (`self.GetAbilityLevel`))
  (bind _returnvalue_2 (`GASSCharacter.GetGASSEquipmentManagerComponent` (`self.GetGASSCharacterFromActorInfo`)))
  (`|ExecutionSequence`
    (:`then_0`
      (`self.K2_HasAuthority`
        (:`True`
          (`/Engine/EditorBlueprintResources/StandardMacros.IsValid` _returnvalue_2
            (:`Is Valid`
              (set `self.EMC` _returnvalue_2)
              (if (< _returnvalue 0)
                (`GASSEquipmentManagerComponent.DisarmItem` (`self.EMC`))
                (else
                  (`GASSEquipmentManagerComponent.ChangeArmItem` (`self.EMC`) (`KismetMathLibrary.Conv_ByteToInt` (`|GetArrayItem` (`self.LevelEquipIndexMapping`) _returnvalue))))))))))
    (:`then_1`
      (`self.K2_EndAbility`))))