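; Gameplay ability for interacting with a storage actor, triggered by an event whose target is the storage.
; On authority, it counts interacting players on the GASSStorage, moves the target open on activation and closes it once the last player's ability ends.
; Without authority, it asynchronously pushes the storage inventory widget to the GameMenu layer and binds its grid to the storage.
; Widget deactivation or failed setup ends the ability, which cancels or removes the widget.
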(event `self.K2_OnEndAbility`
  (params (bWasCancelled :type Boolean))
  (`self.RemoveWidget`)
  (`self.K2_HasAuthority`
    (:`True`
      (bind _asgassstorage (cast `GASSStorage` (`self.StorageActor`)))
      (`GASSStorage.SubCurrentInteractingPlayer` _asgassstorage)
      (bind _returnvalue (`GASSStorage.IsCurrentInteractingPlayerExist` _asgassstorage))
      (if (not _returnvalue)
        ;[1 1 1] Close
        (`self.SetInformationFromMagnitude` 0.0)
        (`self.MoveTargetWithInformation`)))))

(event `self.K2_ActivateAbilityFromEvent`
  (params (EventData :type "GameplayEventData Structure (by ref)"))
  (`self.SetInformationFromEventData` EventData)
  (set `self.StorageActor` (`.Target` (break `GameplayEventData` EventData)))
  (`self.K2_HasAuthority`
    (:`True`
      (bind _asgassstorage (cast `GASSStorage` (`self.StorageActor`)))
      (`GASSStorage.AddCurrentInteractingPlayer` _asgassstorage)
      ;[1 1 1] Open
      (`self.SetInformationFromMagnitude` 1.0)
      (`self.MoveTargetWithInformation`))
    (:`False`
      (`self.CreateAndDisplayWidget`))))

(event `CreateAndDisplayWidget`
  (`/Engine/EditorBlueprintResources/StandardMacros.IsValid` (`self.SpawnedWidget`)
    (:`Is Not Valid`
      (bind (_asynctaskproxy _userwidget) (`AsyncAction_PushContentToLayerForPlayer.PushContentToLayerForPlayer` (`self.GetGASSPlayerControllerFromActorInfo`) "/Game/UI/Inventory/W_Character_Inventory_Storage.W_Character_Inventory_Storage_C" (struct :`TagName` "UI.Layer.GameMenu"))
        (:`then`
          (set `self.AsyncAction_CreateWidget` _asynctaskproxy))
        (:`BeforePush`
          (bind _asw_character_inventory_storage (cast `/Game/UI/Inventory/W_Character_Inventory_Storage` _userwidget)
            (:`then`
              (bind _newparam (`/Game/UI/Inventory/W_Character_Inventory_Storage.GetStorageGrid` _asw_character_inventory_storage))
              (bind _returnvalue (`GASSInventoryGrid.TrySetIMC_Storage` _newparam (`self.StorageActor`)))
              (if (not _returnvalue)
                (`self.RemoveWidget`)
                (`self.K2_EndAbility`)))
            (:`CastFailed`
              (`self.RemoveWidget`)
              (`self.K2_EndAbility`))))
        (:`AfterPush`
          (bind _output_get (set `self.SpawnedWidget` _userwidget))
          (add `CommonActivatableWidget.BP_OnWidgetDeactivated` _output_get (delegate `OnWidgetDeactivated`)))))))

(event `OnWidgetDeactivated`
  (`self.RemoveWidget`)
  (`self.K2_EndAbility`))

(event `RemoveWidget`
  (`|ExecutionSequence`
    (:`then_0`
      (`/Engine/EditorBlueprintResources/StandardMacros.IsValid` (`self.AsyncAction_CreateWidget`)
        (:`Is Valid`
          (`CancellableAsyncAction.Cancel` (`self.AsyncAction_CreateWidget`)))))
    (:`then_1`
      (`/Engine/EditorBlueprintResources/StandardMacros.IsValid` (`self.SpawnedWidget`)
        (:`Is Valid`
          (`CommonActivatableWidget.DeactivateWidget` (`self.SpawnedWidget`))
          (set `self.SpawnedWidget` null))))))