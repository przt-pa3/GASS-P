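; Gameplay ability that handles collecting an interacted item into the player's inventory, triggered by a gameplay event.
; It disables the target's collision, sets a one-second lifespan and executes the Collect gameplay cue.
; On authority, it adds the target's pickup to the instigator controller's inventory manager, then after a short delay destroys the still-valid target and ends.
; The non-authority branch has no explicit EndAbility call.
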(event `self.K2_ActivateAbilityFromEvent`
  (params (EventData :type "GameplayEventData Structure (by ref)"))
  (bind (_eventtag _instigator _target) (break `GameplayEventData` EventData))
  (`Actor.SetActorEnableCollision` _target false)
  (`Actor.SetLifeSpan` _target 1.0)
  (`self.K2_ExecuteGameplayCueWithParams` (struct :`TagName` "GameplayCue.Interact.Collect") (`AbilitySystemBlueprintLibrary.MakeGameplayCueParameters` 0.0 0.0 (struct) (struct) (struct) (struct) (struct) (0.0 0.0 0.0) (0.0 0.0 0.0) _instigator _target _target))
  (`self.K2_HasAuthority`
    (:`True`
      (bind `_as폰` (cast `Pawn` _instigator)
        (:`then`
          (bind _asgassplayer_controller (cast `GASSPlayerController` (`Pawn.GetController` `_as폰`))
            (:`then`
              (`PickupableStatics.AddPickupToInventory` (`GASSPlayerController.GetGASSInventoryManagerComponent` _asgassplayer_controller) (`PickupableStatics.GetFirstPickupableFromActor` _target))
              (`AbilityTask_WaitDelay.WaitDelay` 1.0
                (:`OnFinish`
                  (if (`KismetSystemLibrary.IsValid` _target)
                    (`Actor.K2_DestroyActor` _target)
                    (`self.K2_EndAbility`)))))
            (:`CastFailed`
              (`self.K2_EndAbility` :!label _label))))
        (:`CastFailed`
          (goto _label))))))