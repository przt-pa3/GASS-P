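; GA_Interact_Collect is an interaction gameplay ability that picks up a B_CollectableBase target into the instigator's inventory.
; On event activation, the authority disables the target's collision, then the pickup is added through the GASS player controller's inventory manager component.
; A full add, or a partial one flagged for a cue, fires the Collect GameplayCue.
; Only fully added items are destroyed; otherwise ending the ability restores collision.
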(event `self.K2_OnEndAbility`
  (params (bWasCancelled :type Boolean))
  (bind _targetactor (`self.TargetActor`))
  (if (not (`self.ShouldDestroy`))
    (`/Engine/EditorBlueprintResources/StandardMacros.IsValid` _targetactor
      (:`Is Valid`
        (bind _asb_collectable_base (cast `/Game/Items/B_CollectableBase` _targetactor))
        (`/Game/Items/B_CollectableBase.ClientSetActorEnableCollision` _asb_collectable_base true)))))

(event `self.K2_ActivateAbilityFromEvent`
  (params (EventData :type "GameplayEventData Structure (by ref)"))
  (bind (_eventtag _instigator _target) (break `GameplayEventData` EventData))
  (bind _targetactor (`self.TargetActor`))
  (`|ExecutionSequence`
    (:`then_0`
      (`self.K2_HasAuthority`
        (:`True`
          (set `self.InstigatorActor` _instigator)
          (bind _output_get (set `self.TargetActor` _target))
          (bind _asb_collectable_base (cast `/Game/Items/B_CollectableBase` _output_get))
          (`/Game/Items/B_CollectableBase.ClientSetActorEnableCollision` _asb_collectable_base false)
          (set `self.ShouldDestroy` false))))
    (:`then_1`
      (bind `_as폰` (cast `Pawn` (`self.InstigatorActor`))
        (:`then`
          (bind _asgassplayer_controller (cast `GASSPlayerController` (`Pawn.GetController` `_as폰`))
            (:`then`
              (bind (_iscompletelyadded _shouldsendcue) (`PickupableStatics.AddPickupToInventory` (`GASSPlayerController.GetGASSInventoryManagerComponent` _asgassplayer_controller) (`PickupableStatics.GetFirstPickupableFromActor` (`self.TargetActor`))))
              (bind _output_get_2 (set `self.ShouldDestroy` _iscompletelyadded))
              (if _output_get_2
                (`self.K2_ExecuteGameplayCueWithParams` (struct :`TagName` "GameplayCue.Interact.Collect") (`AbilitySystemBlueprintLibrary.MakeGameplayCueParameters` 0.0 0.0 (struct) (struct) (struct) (struct) (struct) (0.0 0.0 0.0) (0.0 0.0 0.0) (`self.InstigatorActor`) _targetactor _targetactor) :!label _label)
                (if (`self.ShouldDestroy`)
                  (`Actor.K2_DestroyActor` (`self.TargetActor`)))
                (`self.K2_EndAbility`)
                (elif _shouldsendcue
                  (goto _label)
                  (else
                    (`self.K2_EndAbility`)))))
            (:`CastFailed`
              (`self.K2_EndAbility`))))
        (:`CastFailed`
          (`self.K2_EndAbility`))))))