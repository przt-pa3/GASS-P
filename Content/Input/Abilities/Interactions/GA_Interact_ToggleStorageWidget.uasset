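; Gameplay ability that opens the character inventory and storage screen when a player interacts with a storage target.
; Activated by a gameplay event, it pushes the storage widget to the player's GameMenu UI layer through an async CommonUI push.
; Before the push, it hands the event's target to the widget's storage grid as the storage source.
; The ability ends when the widget deactivates.
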(event `self.K2_ActivateAbilityFromEvent`
  (params (EventData :type "GameplayEventData Structure (by ref)"))
  (`KismetSystemLibrary.PrintString` "Toggle Storage Called")
  (`self.CreateAndDisplayWidget`))

(event `CreateAndDisplayWidget`
  (bind (_asynctaskproxy _userwidget) (`AsyncAction_PushContentToLayerForPlayer.PushContentToLayerForPlayer` (`self.GetGASSPlayerControllerFromActorInfo`) "/Game/UI/Inventory/W_Character_Inventory_Storage.W_Character_Inventory_Storage_C" (struct :`TagName` "UI.Layer.GameMenu"))
    (:`BeforePush`
      (bind _asw_character_inventory_storage (cast `/Game/UI/Inventory/W_Character_Inventory_Storage` _userwidget))
      (bind _newparam (`/Game/UI/Inventory/W_Character_Inventory_Storage.GetStorageGrid` _asw_character_inventory_storage))
      (`GASSInventoryGrid.TrySetIMC_Storage` _newparam (`.Target` (break `GameplayEventData` (stale `self.K2_ActivateAbilityFromEvent` EventData)))))
    (:`AfterPush`
      (add `CommonActivatableWidget.BP_OnWidgetDeactivated` _userwidget (delegate `OnWidgetDeactivated`)))))

(event `OnWidgetDeactivated`
  (`self.K2_EndAbility`))